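; BP_RateStar is a score pickup in the SuperGrid tutorial level that awards Points to a BP_Ball.
; On BeginPlay it hides its PickupText widget and fills in the point value, but never shows it here.
; Sphere overlap calls PickUp, which increments the ball's score, plays a sound, destroys the star and prints the total.
; The overlap event also destroys it after a delay, even for non-ball actors.
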(event `self.ReceiveBeginPlay`
  (bind _widget (`self.Widget`))
  (`SceneComponent.SetVisibility` _widget false false)
  (bind _aspickup_text (cast `/Game/UI/PickupText` (`WidgetComponent.GetUserWidgetObject` _widget)))
  (set `/Game/UI/PickupText.ScoreValue` (`self.points`) _aspickup_text))

(event `self.Sphere.OnComponentBeginOverlap`
  (params (OverlappedComponent :type "PrimitiveComponent Object Reference") (OtherActor :type "Actor Object Reference") (OtherComp :type "PrimitiveComponent Object Reference") (OtherBodyIndex :type Integer) (bFromSweep :type Boolean) (SweepResult :type "HitResult Structure (by ref)"))
  (`self.PickUp` OtherActor)
  (`KismetSystemLibrary.Delay` 1.0)
  (`self.K2_DestroyActor`))

(fn `PickUp`
  (params (Object :type "Object Object Reference"))
  ;[1 1 1] Increment Score
  (bind _asbp_ball (cast `/Game/Blueprints/BP_Ball` Object))
  (`/Game/Blueprints/BP_Ball.IncrementScore` _asbp_ball (`self.Points`))
  (`|ExecutionSequence`
    (:`then_0`
      ;[1 1 1] Play Sound
      (`GameplayStatics.PlaySound2D` (`self.PickupSound`) 1.0 1.0 0.0 null null)
      (`self.K2_DestroyActor`))
    (:`then_1`
      (`KismetSystemLibrary.PrintString` (`KismetStringLibrary.Concat_StrStr` "Collected Points " (`KismetStringLibrary.Conv_IntToString` (`/Game/Blueprints/BP_Ball.Score` _asbp_ball))) true true (struct :`G` 0.66 :`B` 1.0 :`A` 1.0) 10.0))))

(fn `UserConstructionScript`)