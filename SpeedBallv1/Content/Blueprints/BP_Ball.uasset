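; BP_Ball is a ball Blueprint that tracks health and score and puts the HUD on screen.
; On BeginPlay it creates the Hud widget and adds it to the viewport.
; AnyDamage subtracts damage from CurrentHealth with no clamp or death check, and IncrementScore adds points to Score.
; GetBallRef returns the ball itself, while GetBallRef2 and the construction script are empty.
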(event `self.ReceiveAnyDamage`
  (params (Damage :type "Float (single-precision)") (DamageType :type "DamageType Object Reference") (InstigatedBy :type "Controller Object Reference") (DamageCauser :type "Actor Object Reference"))
  (set `self.CurrentHealth` (- (`self.CurrentHealth`) Damage)))

(event `self.ReceiveBeginPlay`
  ;[1 1 1] HUD
  (bind _returnvalue (`|CreateWidget` "/Game/UI/Hud.Hud_C"))
  (`UserWidget.AddToViewport` _returnvalue 0))

(fn `GetBallRef`
  (returns (Ball :type "/Game/Blueprints/BP_Ball Object Reference"))
  (return self))

(fn `GetBallRef2`
  (returns (BPBall2 :type "/Game/Blueprints/BP_Ball Object Reference"))
  (return null))

(fn `IncrementScore`
  (params (`P Score` :type Integer))
  (set `self.Score` (+ `P Score` (`self.Score`))))

(fn `UserConstructionScript`)